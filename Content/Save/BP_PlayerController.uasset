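; Player controller that saves and loads the list of destroyed actors between the game instance and a save slot.
; BeginPlay caches the BP_GameInstance reference, and LoadGame retries each tick until it is valid, then copies the saved list into it.
; SaveGame loads the existing BP_SaveGame or creates one, copies the game instance's list into it and writes it to the slot.
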(event `self.ReceiveBeginPlay`
  (bind _asbp_game_instance (cast `/Game/Save/BP_GameInstance` (`GameplayStatics.GetGameInstance`)))
  (set `self.GameInstanceRef` _asbp_game_instance))

(event `LoadGame`
  (`/Engine/EditorBlueprintResources/StandardMacros.IsValid` (`self.GameInstanceRef`) :!label _label
    (:`Is Valid`
      (bind _returnvalue (`GameplayStatics.LoadGameFromSlot` (`self.SlotName`)))
      (bind _asbp_save_game (cast `/Game/Save/BP_SaveGame` _returnvalue))
      (bind _output_get (set `self.SaveGameRef` _asbp_save_game))
      (set `/Game/Save/BP_GameInstance.DestroyedActors` (`/Game/Save/BP_SaveGame.DestroyedActors` _output_get) (`self.GameInstanceRef`)))
    (:`Is Not Valid`
      (`KismetSystemLibrary.DelayUntilNextTick`)
      (goto _label))))

(event `SaveGame`
  (bind _savegameref (`self.SaveGameRef`))
  (bind _returnvalue (`GameplayStatics.DoesSaveGameExist` (`self.SlotName`)))
  (if _returnvalue
    (bind _returnvalue_2 (`GameplayStatics.LoadGameFromSlot` (`self.SlotName`)))
    (bind _asbp_save_game (cast `/Game/Save/BP_SaveGame` _returnvalue_2))
    (set `self.SaveGameRef` _asbp_save_game)
    (else
      (bind _returnvalue_3 (`GameplayStatics.CreateSaveGameObject` "/Game/Save/BP_SaveGame.BP_SaveGame_C"))
      (set `self.SaveGameRef` _returnvalue_3)))
  (set `/Game/Save/BP_SaveGame.DestroyedActors` (`/Game/Save/BP_GameInstance.DestroyedActors` (`self.GameInstanceRef`)) _savegameref)
  (`GameplayStatics.SaveGameToSlot` _savegameref (`self.SlotName`)))

(fn `UserConstructionScript`)