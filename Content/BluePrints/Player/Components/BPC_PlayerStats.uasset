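; Player component that manages health, stamina, dash charges, coins, diamonds and saved location in a stats struct, pushing changes to the HUD.
; BeginPlay retries until the character exists, then loads data via BP_GameInstance, refreshes the HUD, restores location and initializes equipment.
; Looping timers regenerate stamina and dash charges, clearing themselves when full.
; DecreaseHealth returns true on lethal damage and resets health to a fixed value instead of zero.
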(event `self.ReceiveBeginPlay`
  (`/Engine/EditorBlueprintResources/StandardMacros.IsValid` (`GameplayStatics.GetPlayerCharacter` 0) :!label _label
    (:`Is Valid`
      (bind _asbp_game_instance (cast `/Game/BluePrints/BP_GameInstance` (`GameplayStatics.GetGameInstance`)))
      (`/Game/BluePrints/BP_GameInstance.LoadPlayerData` _asbp_game_instance)
      (bind _asbp_player_controller (cast `/Game/BluePrints/BP_PlayerController` (`GameplayStatics.GetPlayerController` 0)))
      (set `self.HUDRef` (`/Game/BluePrints/BP_PlayerController.MainWidgetRef` _asbp_player_controller))
      (`self.UpdatePlayerStats`)
      (bind _asbp_player_character (cast `/Game/BluePrints/Player/BP_PlayerCharacter` (`GameplayStatics.GetPlayerCharacter` 0)))
      (`/Game/BluePrints/Player/Components/BPC_EquipmentSystem.Init` (`/Game/BluePrints/Player/BP_PlayerCharacter.BPC_EquipmentSystem` _asbp_player_character)))
    (:`Is Not Valid`
      (`KismetSystemLibrary.K2_SetTimerDelegate` (delegate `Init`) 0.01))))

(event `Init`
  (goto _label))

(event `RecoverStamina`
  (bind _returnvalue (`KismetSystemLibrary.K2_SetTimer` null "IncreaseStamina" 0.01 true))
  (set `self.StaminaLoop` _returnvalue))

(event `RecoverDash`
  (`self.UpdateDashBar`)
  (bind _returnvalue (`KismetSystemLibrary.K2_SetTimer` null "RegenerateDash" 0.01 true (`.InitialDashRegenDelay_28_B00BAED74F222C91D2ADD89DF257C416` (break `/Game/BluePrints/Structures/S_PlayerStats` (`self.PlayerStatsData`)))))
  (set `self.DashLoop` _returnvalue))

(fn `DecreaseHealth`
  (params (Damage :type "Float (double-precision)"))
  (returns (`Death?` :type Boolean))
  (bind _playerstatsdata (`self.PlayerStatsData`))
  (bind _returnvalue (- (`.CurrentHealth_5_98BB0FFC47C134DAA92996808D1B4AA0` (break `/Game/BluePrints/Structures/S_PlayerStats` _playerstatsdata)) Damage))
  (if (> _returnvalue 0.0)
    (setmembers `/Game/BluePrints/Structures/S_PlayerStats` :`StructRef` _playerstatsdata :`CurrentHealth` _returnvalue)
    (`self.UpdateHealthBar`)
    (return false)
    (else
      (setmembers `/Game/BluePrints/Structures/S_PlayerStats` :`StructRef` _playerstatsdata :`CurrentHealth` 70.0)
      (`self.UpdateHealthBar`)
      (return true))))

(fn `DecreaseStamina`
  (params (DrainAmount :type "Float (double-precision)"))
  (bind _playerstatsdata (`self.PlayerStatsData`))
  (`KismetSystemLibrary.K2_ClearAndInvalidateTimerHandle` (`self.StaminaLoop`))
  (setmembers `/Game/BluePrints/Structures/S_PlayerStats` :`StructRef` _playerstatsdata :`CurrentStamina` (- (`.CurrentStamina_9_21289666469E874A0282E3B5143972BC` (break `/Game/BluePrints/Structures/S_PlayerStats` _playerstatsdata)) DrainAmount))
  (`self.UpdateStaminaBar`))

(fn `IncreaseHealth`
  (params (IncreaseAmount :type "Float (double-precision)"))
  (bind _playerstatsdata (`self.PlayerStatsData`))
  (bind ((`PlayerLocation_33_5B6E195A49F61389113A06B498A20BB3` _playerlocation) (`CurrentHealth_5_98BB0FFC47C134DAA92996808D1B4AA0` _currenthealth) (`MaxHealth_7_AB1A1C134EAC27803A09DAAFC4F0611C` _maxhealth)) (break `/Game/BluePrints/Structures/S_PlayerStats` (`self.PlayerStatsData`)))
  (bind _returnvalue (+ IncreaseAmount _currenthealth))
  (if (>= _returnvalue _maxhealth)
    (setmembers `/Game/BluePrints/Structures/S_PlayerStats` :`StructRef` _playerstatsdata :`CurrentHealth` _maxhealth)
    (else
      (setmembers `/Game/BluePrints/Structures/S_PlayerStats` :`StructRef` _playerstatsdata :`CurrentHealth` _returnvalue)))
  (`self.UpdateHealthBar`))

(fn `IncreaseMaxHealth`
  (params (IncreaseAmount :type "Float (double-precision)"))
  (bind _playerstatsdata (`self.PlayerStatsData`))
  (bind ((`PlayerLocation_33_5B6E195A49F61389113A06B498A20BB3` _playerlocation) (`CurrentHealth_5_98BB0FFC47C134DAA92996808D1B4AA0` _currenthealth) (`MaxHealth_7_AB1A1C134EAC27803A09DAAFC4F0611C` _maxhealth)) (break `/Game/BluePrints/Structures/S_PlayerStats` _playerstatsdata))
  (setmembers `/Game/BluePrints/Structures/S_PlayerStats` :`StructRef` _playerstatsdata :`CurrentHealth` (+ IncreaseAmount _currenthealth) :`MaxHealth` (+ IncreaseAmount _maxhealth))
  (`self.UpdateHealthBar`))

(fn `IncreaseMaxStamina`
  (params (IncreaseAmount :type "Float (double-precision)"))
  (bind _playerstatsdata (`self.PlayerStatsData`))
  (bind ((`PlayerLocation_33_5B6E195A49F61389113A06B498A20BB3` _playerlocation) (`CurrentStamina_9_21289666469E874A0282E3B5143972BC` _currentstamina) (`MaxStamina_11_F1D35E4F4127AC4B12BE4CB040CA9CA2` _maxstamina)) (break `/Game/BluePrints/Structures/S_PlayerStats` _playerstatsdata))
  (setmembers `/Game/BluePrints/Structures/S_PlayerStats` :`StructRef` _playerstatsdata :`CurrentStamina` (+ IncreaseAmount _currentstamina) :`MaxStamina` (+ IncreaseAmount _maxstamina))
  (`self.UpdateStaminaBar`))

(fn `IncreaseStamina`
  (bind _playerstatsdata (`self.PlayerStatsData`))
  (bind ((`CurrentStamina_9_21289666469E874A0282E3B5143972BC` _currentstamina) (`MaxStamina_11_F1D35E4F4127AC4B12BE4CB040CA9CA2` _maxstamina)) (break `/Game/BluePrints/Structures/S_PlayerStats` (`self.PlayerStatsData`)))
  (bind _returnvalue (+ (`self.Increase Amount`) _currentstamina))
  (if (>= _returnvalue _maxstamina)
    (setmembers `/Game/BluePrints/Structures/S_PlayerStats` :`StructRef` _playerstatsdata :`CurrentStamina` _maxstamina)
    (`KismetSystemLibrary.K2_ClearAndInvalidateTimerHandle` (`self.StaminaLoop`))
    (else
      (setmembers `/Game/BluePrints/Structures/S_PlayerStats` :`StructRef` _playerstatsdata :`CurrentStamina` _returnvalue)))
  (`self.UpdateStaminaBar`))

(fn `RegenerateDash`
  (bind _playerstatsdata (`self.PlayerStatsData`))
  (bind ((`CurrentDash_20_49ED6CEC4752BD05727CC2827D5D19B5` _currentdash) (`MaxDash_22_68AD41564F8F34B3B1F63A817B77849E` _maxdash) (`RegenDashProgress_29_36B61846444DC7D7916380AFA6B4AC91` _regendashprogress)) (break `/Game/BluePrints/Structures/S_PlayerStats` (`self.PlayerStatsData`)))
  (bind _returnvalue (+ _regendashprogress (`self.Regenerate Amount`)))
  (if (< _currentdash _maxdash)
    (if (>= _returnvalue 100.0)
      (setmembers `/Game/BluePrints/Structures/S_PlayerStats` :`StructRef` _playerstatsdata :`RegenDashProgress` 0.0)
      (`/Engine/EditorBlueprintResources/StandardMacros.IncrementInt` (`.CurrentDash_20_49ED6CEC4752BD05727CC2827D5D19B5` (break `/Game/BluePrints/Structures/S_PlayerStats` _playerstatsdata))
        (:`  `
          _))
      (else
        (setmembers `/Game/BluePrints/Structures/S_PlayerStats` :`StructRef` _playerstatsdata :`RegenDashProgress` _returnvalue)))
    (else
      (`KismetSystemLibrary.K2_ClearAndInvalidateTimerHandle` (`self.DashLoop`))))
  (`self.UpdateDashBar`))

(fn `UpdateCoins`
  (params (ChangeAmount :type Integer))
  (bind _playerstatsdata (`self.PlayerStatsData`))
  (setmembers `/Game/BluePrints/Structures/S_PlayerStats` :`StructRef` _playerstatsdata :`Coins` (+ ChangeAmount (`.Coins_14_F41C27064E96CB3AA899418D09EF6177` (break `/Game/BluePrints/Structures/S_PlayerStats` _playerstatsdata))))
  (`self.UpdateCoinsWidget`))

(fn `UpdateCoinsWidget`
  (set `TextBlock.Text` (`KismetTextLibrary.Conv_IntToText` (`.Coins_14_F41C27064E96CB3AA899418D09EF6177` (break `/Game/BluePrints/Structures/S_PlayerStats` (`self.PlayerStatsData`)))) (`/Game/UI/MainGame/WB_HUD.CoinAmount` (`self.HUDRef`))))

(fn `UpdateDashBar`
  (bind _hudref (`self.HUDRef`))
  (bind _playerstatsdata (`self.PlayerStatsData`))
  (bind ((`PlayerLocation_33_5B6E195A49F61389113A06B498A20BB3` _playerlocation) (`RegenDashProgress_29_36B61846444DC7D7916380AFA6B4AC91` _regendashprogress)) (break `/Game/BluePrints/Structures/S_PlayerStats` _playerstatsdata))
  (`/Game/UI/RoundProgressBar/WB_RoundProgressBar.SetDashPercent` (`/Game/UI/MainGame/WB_HUD.DashBarProg` _hudref) (`KismetMathLibrary.SelectFloat` (/ _regendashprogress 100.0) 1.0 (!= _regendashprogress 0.0)))
  (`TextBlock.SetText` (`/Game/UI/MainGame/WB_HUD.DashAmount` _hudref) (`KismetTextLibrary.Conv_IntToText` (`.CurrentDash_20_49ED6CEC4752BD05727CC2827D5D19B5` (break `/Game/BluePrints/Structures/S_PlayerStats` _playerstatsdata)))))

(fn `UpdateDiamonds`
  (params (ChangeAmount :type Integer))
  (bind _playerstatsdata (`self.PlayerStatsData`))
  (setmembers `/Game/BluePrints/Structures/S_PlayerStats` :`StructRef` _playerstatsdata :`Diamonds` (+ ChangeAmount (`.Diamonds_16_88917EBA486C83AC451AA3B1E6FAAD89` (break `/Game/BluePrints/Structures/S_PlayerStats` _playerstatsdata))))
  (`self.UpdateDiamondsWidget`))

(fn `UpdateDiamondsWidget`
  (set `TextBlock.Text` (`KismetTextLibrary.Conv_IntToText` (`.Diamonds_16_88917EBA486C83AC451AA3B1E6FAAD89` (break `/Game/BluePrints/Structures/S_PlayerStats` (`self.PlayerStatsData`)))) (`/Game/UI/MainGame/WB_HUD.DiamondAmount` (`self.HUDRef`))))

(fn `UpdateHealthBar`
  (bind ((`PlayerLocation_33_5B6E195A49F61389113A06B498A20BB3` _playerlocation) (`CurrentHealth_5_98BB0FFC47C134DAA92996808D1B4AA0` _currenthealth) (`MaxHealth_7_AB1A1C134EAC27803A09DAAFC4F0611C` _maxhealth)) (break `/Game/BluePrints/Structures/S_PlayerStats` (`self.PlayerStatsData`)))
  (`ProgressBar.SetPercent` (`/Game/UI/MainGame/WB_HUD.HealthBar` (`self.HUDRef`)) (/ _currenthealth _maxhealth)))

(fn `UpdatePlayerStats`
  (`self.UpdateHealthBar`)
  (`self.UpdateCoins` 0)
  (`self.UpdateDiamonds` 0)
  (`self.RecoverStamina`)
  (`self.RecoverDash`)
  (bind _asbp_player_character (cast `/Game/BluePrints/Player/BP_PlayerCharacter` (`GameplayStatics.GetPlayerCharacter` 0)))
  (`Actor.K2_SetActorTransform` _asbp_player_character (`.PlayerLocation_33_5B6E195A49F61389113A06B498A20BB3` (break `/Game/BluePrints/Structures/S_PlayerStats` (`self.PlayerStatsData`))) false false))

(fn `UpdateStaminaBar`
  (bind ((`CurrentStamina_9_21289666469E874A0282E3B5143972BC` _currentstamina) (`MaxStamina_11_F1D35E4F4127AC4B12BE4CB040CA9CA2` _maxstamina)) (break `/Game/BluePrints/Structures/S_PlayerStats` (`self.PlayerStatsData`)))
  (`ProgressBar.SetPercent` (`/Game/UI/MainGame/WB_HUD.StaminaBar` (`self.HUDRef`)) (/ _currentstamina _maxstamina)))