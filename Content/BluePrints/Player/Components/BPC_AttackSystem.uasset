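; Player attack component that handles light, heavy and three-step unarmed combo input, drawing a sheathed weapon first.
; Repeat presses set chain flags, and ResetAttack clears them before delayed stamina recovery.
; Socket-based sphere traces for punches and kicks apply damage once per listed enemy.
; Attack, ChainAttacks and CalculateDamage are empty; the stamina-gated logic dispatching to weapon or unarmed attacks is disconnected.
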(event `self.ReceiveBeginPlay`
  ;[0.05098 0.05098 0.05098] Set References
  (bind _asbp_player_character (cast `/Game/BluePrints/Player/BP_PlayerCharacter` (`self.GetOwner`)))
  (bind _output_get (set `self.CharRef` _asbp_player_character))
  (set `self.MeshRef` (`Character.Mesh` _output_get))
  (set `self.EquipmentSystem` (`/Game/BluePrints/Player/BP_PlayerCharacter.BPC_EquipmentSystem` _output_get))
  (set `self.PlayerStats` (`/Game/BluePrints/Player/BP_PlayerCharacter.BPC_PlayerStats` _output_get)))

(event `CalculateDamage`
  ;[0.8671 1 0] Modify Damage
)

(event `EnhancedInput|/Game/Input/Actions/IA_LightAttack`
  (params (ActionValue :type Boolean) (ElapsedSeconds :type "Float (double-precision)") (TriggeredSeconds :type "Float (double-precision)") (InputAction :type "InputAction Object Reference" :default "/Game/Input/Actions/IA_LightAttack.IA_LightAttack"))
  (bind _equipmentsystem (`self.EquipmentSystem`))
  ;[0.05098 0.05098 0.05098] Light / Heavy Attack Input
  (:`Started`
    (if (not (`self.CannotAttack`))
      (`/Engine/EditorBlueprintResources/StandardMacros.IsValid` (`/Game/BluePrints/Player/Components/BPC_EquipmentSystem.EquippedWeapon` _equipmentsystem)
        (:`Is Valid`
          (if (`/Game/BluePrints/Player/Components/BPC_EquipmentSystem.isWeaponDrawn?` _equipmentsystem)
            (if (or (`self.LightAttack`) (`self.HeavyAttack`))
              (set `self.ChainAttack` true)
              (set `self.LightAttack` true)
              (set `self.HeavyAttack` false)
              (else
                (set `self.LightAttack` true)
                (set `self.HeavyAttack` false)
                (`self.Attack`)))
            (else
              (`/Game/BluePrints/Player/Components/BPC_EquipmentSystem.Draw/Sheath` _equipmentsystem :!label _label))))
        (:`Is Not Valid`
          (if (`self.NoWeapon`) :!label _label_2
            (set `self.ChainAttack` true)
            (else
              (set `self.NoWeapon` true)
              (`self.Attack`))))))))

(event `EnhancedInput|/Game/Input/Actions/IA_HeavyAttack`
  (params (ActionValue :type Boolean) (ElapsedSeconds :type "Float (double-precision)") (TriggeredSeconds :type "Float (double-precision)") (InputAction :type "InputAction Object Reference" :default "/Game/Input/Actions/IA_HeavyAttack.IA_HeavyAttack"))
  (bind _equipmentsystem (`self.EquipmentSystem`))
  ;[0.05098 0.05098 0.05098] Light / Heavy Attack Input
  (:`Started`
    (if (not (`self.CannotAttack`))
      (`/Engine/EditorBlueprintResources/StandardMacros.IsValid` (`/Game/BluePrints/Player/Components/BPC_EquipmentSystem.EquippedWeapon` _equipmentsystem)
        (:`Is Valid`
          (if (`/Game/BluePrints/Player/Components/BPC_EquipmentSystem.isWeaponDrawn?` _equipmentsystem)
            (if (or (`self.LightAttack`) (`self.HeavyAttack`))
              (set `self.ChainAttack` true)
              (set `self.LightAttack` false)
              (set `self.HeavyAttack` true)
              (else
                (set `self.LightAttack` false)
                (set `self.HeavyAttack` true)
                (`self.Attack`)))
            (else
              (goto _label))))
        (:`Is Not Valid`
          (goto _label_2))))))

(event `Attack`
  ;[0.05098 0.05098 0.05098] Attack Logic
)

(event `ChainAttacks`
  ;[0.05098 0.05098 0.05098] Attack Logic
)

(event `ResetAttack`
  ;[0.05098 0.05098 0.05098] Atack End
  (`self.ResetVariablesToDefault`)
  (`KismetSystemLibrary.Delay` 1.2)
  (set `self.CannotAttack` false)
  (`KismetSystemLibrary.Delay` 0.8)
  (if (not (`self.isAttacking?`))
    (`/Game/BluePrints/Player/Components/BPC_PlayerStats.RecoverStamina` (`self.PlayerStats`))))

(event `RightAttackTrace`
  (bind _meshref (`self.MeshRef`))
  (bind _returnvalue (`SceneComponent.GetSocketLocation` _meshref "spine_05"))
  ;[0.05098 0.05098 0.05098] No Weapon Attack Traces
  ;;[0.05098 0.05098 0.05098] Right Attack
  (bind (_outhit _returnvalue_2) (`KismetSystemLibrary.SphereTraceSingleForObjects` _returnvalue (`KismetMathLibrary.MakeVector` (.x (`SceneComponent.GetSocketLocation` _meshref "hand_r")) (.y _returnvalue) (.z (`SceneComponent.GetSocketLocation` _meshref "hand_r"))) 5.0 (`|MakeArray` "ObjectTypeQuery6" :!type "EObjectTypeQuery Enum") true (`|MakeArray` (`self.CharRef`) :!type "Actor Object Reference") "ForDuration" true (struct :`R` 1.0 :`A` 1.0) (struct :`G` 1.0 :`A` 1.0) 0.3))
  (if _returnvalue_2
    (`self.Hit` _outhit)))

(event `NoWeaponAttack`
  (bind _noweaponchainattack (`self.NoWeaponChainAttack`))
  (bind _charref (`self.CharRef`))
  (bind _noweaponchainattack_2 (`self.NoWeaponChainAttack`))
  (bind _output (`|GetArrayItem` (`self.Montage to Play`) _noweaponchainattack))
  ;[0.05098 0.05098 0.05098] No Weapon Combo
  (switch `int` _noweaponchainattack
    (:`0`
      (`Character.PlayAnimMontage` _charref _output 1.0 "None")
      (`/Engine/EditorBlueprintResources/StandardMacros.IncrementInt` _noweaponchainattack_2))
    (:`1`
      (`Character.PlayAnimMontage` _charref _output 1.0 "None")
      (`/Engine/EditorBlueprintResources/StandardMacros.IncrementInt` _noweaponchainattack_2))
    (:`2`
      (`Character.PlayAnimMontage` _charref _output 1.0 "None"))))

(event `NoWeaponAttackStats`
  (bind _noweaponchainattack (`self.NoWeaponChainAttack`))
  (bind _output (`|GetArrayItem` (`self.AttackCosts`) _noweaponchainattack))
  (bind _output_2 (`|GetArrayItem` (`self.AttackDamage`) _noweaponchainattack))
  ;[0.05098 0.05098 0.05098] No Weapon Attack Stats
  (switch `int` _noweaponchainattack
    (:`0`
      (set `self.CurrentAttackCost` _output)
      (set `self.CurrentAttackDamage` _output_2))
    (:`1`
      (set `self.CurrentAttackCost` _output)
      (set `self.CurrentAttackDamage` _output_2))
    (:`2`
      (set `self.CurrentAttackCost` _output)
      (set `self.CurrentAttackDamage` _output_2))))

(event `LeftAttackTrace`
  (bind _meshref (`self.MeshRef`))
  (bind _returnvalue (`SceneComponent.GetSocketLocation` _meshref "spine_05"))
  ;[0.05098 0.05098 0.05098] No Weapon Attack Traces
  ;;[0.05098 0.05098 0.05098] Left Attack
  (bind (_outhit _returnvalue_2) (`KismetSystemLibrary.SphereTraceSingleForObjects` _returnvalue (`KismetMathLibrary.MakeVector` (.x (`SceneComponent.GetSocketLocation` _meshref "hand_l")) (.y _returnvalue) (.z (`SceneComponent.GetSocketLocation` _meshref "hand_l"))) 5.0 (`|MakeArray` "ObjectTypeQuery6" :!type "EObjectTypeQuery Enum") true (`|MakeArray` (`self.CharRef`) :!type "Actor Object Reference") "ForDuration" true (struct :`R` 1.0 :`A` 1.0) (struct :`G` 1.0 :`A` 1.0) 0.3))
  (if _returnvalue_2
    (`self.Hit` _outhit)))

(event `KickAttackTrace`
  (bind _meshref (`self.MeshRef`))
  (bind _returnvalue (`SceneComponent.GetSocketLocation` _meshref "spine_01"))
  ;[0.05098 0.05098 0.05098] No Weapon Attack Traces
  ;;[0.05098 0.05098 0.05098] Kick Attack
  (bind (_outhit _returnvalue_2) (`KismetSystemLibrary.SphereTraceSingleForObjects` _returnvalue (`KismetMathLibrary.MakeVector` (.x (`SceneComponent.GetSocketLocation` _meshref "foot_r")) (.y _returnvalue) (.z (`SceneComponent.GetSocketLocation` _meshref "foot_r"))) 5.0 (`|MakeArray` "ObjectTypeQuery6" :!type "EObjectTypeQuery Enum") true (`|MakeArray` (`self.CharRef`) :!type "Actor Object Reference") "ForDuration" true (struct :`R` 1.0 :`A` 1.0) (struct :`G` 1.0 :`A` 1.0) 0.3))
  (if _returnvalue_2
    (`self.Hit` _outhit)))

(event `Hit`
  (params (Hit :type "HitResult Structure"))
  ;[0.05098 0.05098 0.05098] Hit Enemy
  (bind _enemyref (message `/Game/BluePrints/Interfaces/BPI_DealingDamage.GetEnemyRef` (`.HitActor` (`GameplayStatics.BreakHitResult` Hit))))
  (`/Engine/EditorBlueprintResources/StandardMacros.IsValid` _enemyref
    (:`Is Valid`
      (if (not (`KismetArrayLibrary.Array_Contains` (`self.AlreadyDamagedEnemy`) _enemyref))
        (`KismetArrayLibrary.Array_Add` (`self.AlreadyDamagedEnemy`) _enemyref)
        (`self.CalculateDamage`)
        (`GameplayStatics.ApplyDamage` _enemyref (`self.CurrentAttackDamage`))))))

(fn `EnoughStamina?`
  (params (AttackCost :type "Float (double-precision)"))
  (returns (CanAttack :type Boolean))
  (return (<= AttackCost (`.CurrentStamina_9_21289666469E874A0282E3B5143972BC` (break `/Game/BluePrints/Structures/S_PlayerStats` (`/Game/BluePrints/Player/Components/BPC_PlayerStats.PlayerStatsData` (`self.PlayerStats`)))))))

(fn `KickHitTrace`
  (returns (`Hit?` :type Boolean) (HitActor :type "Actor Object Reference"))
  (bind _meshref (`self.MeshRef`))
  (bind (_outhit _returnvalue) (`KismetSystemLibrary.SphereTraceSingle` :`Start` (`SceneComponent.GetSocketLocation` _meshref "pelvis") :`End` (`SceneComponent.GetSocketLocation` _meshref "foot_r") :`Radius` 12.0 :`TraceChannel` "TraceTypeQuery1" :`DrawTime` 2.0))
  (if _returnvalue
    (if (not (`Actor.ActorHasTag` (`.HitActor` (`GameplayStatics.BreakHitResult` _outhit)) "CanDamage"))
      (return false null))
    (else
      (return false null))))

(fn `PunchHitTrace`
  (returns (`Hit?` :type Boolean) (HitActor :type "Actor Object Reference"))
  (bind _rootcomponent (`Actor.RootComponent` (`self.CharRef`)))
  (bind _returnvalue (`SceneComponent.K2_GetComponentLocation` _rootcomponent))
  (bind (_outhit _returnvalue_2) (`KismetSystemLibrary.SphereTraceSingle` :`Start` _returnvalue :`End` (+ _returnvalue (* (`KismetMathLibrary.GetForwardVector` (`SceneComponent.K2_GetComponentRotation` _rootcomponent)) 90.0)) :`Radius` 12.0 :`TraceChannel` "TraceTypeQuery1" :`DrawTime` 2.0))
  (if _returnvalue_2
    (if (not (`Actor.ActorHasTag` (`.HitActor` (`GameplayStatics.BreakHitResult` _outhit)) "CanDamage"))
      (return false null))
    (else
      (return false null))))

(fn `ResetVariablesToDefault`
  (set `self.isAttacking?` false)
  (set `self.NoWeapon` false)
  (set `self.LightAttack` false)
  (set `self.HeavyAttack` false)
  (set `self.LastAtack?` false)
  (set `self.ChainAttack` false)
  (set `self.NoWeaponChainAttack` 0)
  (set `self.LightChainAttack` 0)
  (set `self.HeavyChainAttack` 0)
  (set `/Game/BluePrints/Player/BP_PlayerCharacter.isPlayingAnimation?` false (`self.CharRef`)))