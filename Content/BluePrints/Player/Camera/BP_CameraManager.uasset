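; BP_CameraManager is a camera actor that smoothly follows a target each frame.
; Tick calls UpdateCameraPosition, which eases the actor toward the FollowTarget's X and Y with VInterpTo while keeping its own height.
; A look-ahead from the target's forward vector, scaled by CameraOffset, shifts the goal along world X only.
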(event `self.ReceiveTick`
  (params (DeltaSeconds :type "Float (single-precision)"))
  (`self.UpdateCameraPosition`))

(fn `UpdateCameraPosition`
  (locals (MoveDirection :type "Vector Structure" :default (0.0 0.0 0.0)))
  (bind (_returnvalue_x _returnvalue_y _returnvalue_z) (`KismetMathLibrary.BreakVector` (`self.K2_GetActorLocation`)))
  (bind _followtarget (`self.FollowTarget`))
  (bind (_returnvalue_x_2 _returnvalue_y_2) (`KismetMathLibrary.BreakVector` (`self.K2_GetActorLocation` _followtarget)))
  (bind _returnvalue_x_3 (`KismetMathLibrary.BreakVector` (* (`self.GetActorForwardVector` _followtarget) (`self.CameraOffset`))))
  (`self.K2_SetActorLocation` (`KismetMathLibrary.VInterpTo` (`self.K2_GetActorLocation`) (+ (`KismetMathLibrary.MakeVector` _returnvalue_x_2 _returnvalue_y_2 _returnvalue_z) (`KismetMathLibrary.MakeVector` _returnvalue_x_3)) (`GameplayStatics.GetWorldDeltaSeconds`) (`self.CameraInterpSpeed`))))

(fn `UserConstructionScript`)