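; Base melee weapon Blueprint for the player character, providing light and heavy attack chains of up to four steps.
; Stats events copy the current step's cost and damage into the character's BPCAttackSystem.
; Attack events play that step's montage, call combo hooks meant for child weapons, then advance the chain.
; AttackTrace runs short debug-drawn line traces from nine cached collision points, passing Pawn hits to the attack system.
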(event `self.ReceiveBeginPlay`
  ;[0.05098 0.05098 0.05098] Set Character Ref
  (bind _asbp_player_character (cast `/Game/BluePrints/Player/BP_PlayerCharacter` (`GameplayStatics.GetPlayerCharacter` 0)))
  (set `self.CharRef` _asbp_player_character))

(event `ComboLightAttack`
  (params (ChainLightAttack :type Integer))
  ;[0.05098 0.05098 0.05098] Combo Logic - Modify in Weapon Childs
)

(event `ComboHeavyAttack`
  (params (ChainHeavyAttack :type Integer))
  ;[0.05098 0.05098 0.05098] Combo Logic - Modify in Weapon Childs
)

(event `LightAttackStats`
  (bind _bpc_attacksystem (`/Game/BluePrints/Player/BP_PlayerCharacter.BPC_AttackSystem` (`self.CharRef`)))
  (bind _lightchainattack (`/Game/BluePrints/Player/Components/BPC_AttackSystem.LightChainAttack` (`/Game/BluePrints/Player/BP_PlayerCharacter.BPC_AttackSystem` (`self.CharRef`))))
  (bind _output (`|GetArrayItem` (`self.LightAttackDamage`) _lightchainattack))
  (bind _output_2 (`|GetArrayItem` (`self.LightAttackCosts`) _lightchainattack))
  ;[0.05098 0.05098 0.05098] Light Attack Stats
  (switch `int` _lightchainattack
    (:`0`
      (set `/Game/BluePrints/Player/Components/BPC_AttackSystem.CurrentAttackCost` _output_2 _bpc_attacksystem)
      (set `/Game/BluePrints/Player/Components/BPC_AttackSystem.CurrentAttackDamage` _output _bpc_attacksystem))
    (:`1`
      (set `/Game/BluePrints/Player/Components/BPC_AttackSystem.CurrentAttackCost` _output_2 _bpc_attacksystem)
      (set `/Game/BluePrints/Player/Components/BPC_AttackSystem.CurrentAttackDamage` _output _bpc_attacksystem))
    (:`2`
      (set `/Game/BluePrints/Player/Components/BPC_AttackSystem.CurrentAttackCost` _output_2 _bpc_attacksystem)
      (set `/Game/BluePrints/Player/Components/BPC_AttackSystem.CurrentAttackDamage` _output _bpc_attacksystem))
    (:`3`
      (set `/Game/BluePrints/Player/Components/BPC_AttackSystem.CurrentAttackCost` _output_2 _bpc_attacksystem)
      (set `/Game/BluePrints/Player/Components/BPC_AttackSystem.CurrentAttackDamage` _output _bpc_attacksystem))))

(event `LightAttack`
  (bind _charref (`self.CharRef`))
  (bind _lightchainattack (`/Game/BluePrints/Player/Components/BPC_AttackSystem.LightChainAttack` (`/Game/BluePrints/Player/BP_PlayerCharacter.BPC_AttackSystem` (`self.CharRef`))))
  (bind _lightchainattack_2 (`/Game/BluePrints/Player/Components/BPC_AttackSystem.LightChainAttack` (`/Game/BluePrints/Player/BP_PlayerCharacter.BPC_AttackSystem` (`self.CharRef`))))
  (bind _output (`|GetArrayItem` (`self.LightAttacks`) _lightchainattack))
  ;[0.05098 0.05098 0.05098] Light Attack Logic
  (switch `int` _lightchainattack
    (:`0`
      (`Character.PlayAnimMontage` _charref _output 1.0 "None")
      (`self.ComboLightAttack` _lightchainattack_2)
      (`/Engine/EditorBlueprintResources/StandardMacros.IncrementInt` _lightchainattack_2))
    (:`1`
      (`Character.PlayAnimMontage` _charref _output 1.0 "None")
      (`self.ComboLightAttack` _lightchainattack_2)
      (`/Engine/EditorBlueprintResources/StandardMacros.IncrementInt` _lightchainattack_2))
    (:`2`
      (`Character.PlayAnimMontage` _charref _output 1.0 "None")
      (`self.ComboLightAttack` _lightchainattack_2)
      (`/Engine/EditorBlueprintResources/StandardMacros.IncrementInt` _lightchainattack_2))
    (:`3`
      (`Character.PlayAnimMontage` _charref _output 1.0 "None")
      (`self.ComboLightAttack` _lightchainattack_2)
      (`/Engine/EditorBlueprintResources/StandardMacros.IncrementInt` _lightchainattack_2))))

(event `HeavyAttackStats`
  (bind _bpc_attacksystem (`/Game/BluePrints/Player/BP_PlayerCharacter.BPC_AttackSystem` (`self.CharRef`)))
  (bind _heavychainattack (`/Game/BluePrints/Player/Components/BPC_AttackSystem.HeavyChainAttack` (`/Game/BluePrints/Player/BP_PlayerCharacter.BPC_AttackSystem` (`self.CharRef`))))
  (bind _output (`|GetArrayItem` (`self.HeavyAttackDamage`) _heavychainattack))
  (bind _output_2 (`|GetArrayItem` (`self.HeavyAttackCosts`) _heavychainattack))
  ;[0.05098 0.05098 0.05098] Heavy Attack Stats
  (switch `int` _heavychainattack
    (:`0`
      (set `/Game/BluePrints/Player/Components/BPC_AttackSystem.CurrentAttackCost` _output_2 _bpc_attacksystem)
      (set `/Game/BluePrints/Player/Components/BPC_AttackSystem.CurrentAttackDamage` _output _bpc_attacksystem))
    (:`1`
      (set `/Game/BluePrints/Player/Components/BPC_AttackSystem.CurrentAttackCost` _output_2 _bpc_attacksystem)
      (set `/Game/BluePrints/Player/Components/BPC_AttackSystem.CurrentAttackDamage` _output _bpc_attacksystem))
    (:`2`
      (set `/Game/BluePrints/Player/Components/BPC_AttackSystem.CurrentAttackCost` _output_2 _bpc_attacksystem)
      (set `/Game/BluePrints/Player/Components/BPC_AttackSystem.CurrentAttackDamage` _output _bpc_attacksystem))
    (:`3`
      (set `/Game/BluePrints/Player/Components/BPC_AttackSystem.CurrentAttackCost` _output_2 _bpc_attacksystem)
      (set `/Game/BluePrints/Player/Components/BPC_AttackSystem.CurrentAttackDamage` _output _bpc_attacksystem))))

(event `HeavyAttack`
  (bind _charref (`self.CharRef`))
  (bind _heavychainattack (`/Game/BluePrints/Player/Components/BPC_AttackSystem.HeavyChainAttack` (`/Game/BluePrints/Player/BP_PlayerCharacter.BPC_AttackSystem` (`self.CharRef`))))
  (bind _heavychainattack_2 (`/Game/BluePrints/Player/Components/BPC_AttackSystem.HeavyChainAttack` (`/Game/BluePrints/Player/BP_PlayerCharacter.BPC_AttackSystem` (`self.CharRef`))))
  (bind _output (`|GetArrayItem` (`self.HeavyAttacks`) _heavychainattack_2))
  ;[0.05098 0.05098 0.05098] Heavy Attack Logic
  (switch `int` _heavychainattack_2
    (:`0`
      (`Character.PlayAnimMontage` _charref _output 1.0 "None")
      (`self.ComboHeavyAttack` _heavychainattack)
      (`/Engine/EditorBlueprintResources/StandardMacros.IncrementInt` _heavychainattack))
    (:`1`
      (`Character.PlayAnimMontage` _charref _output 1.0 "None")
      (`self.ComboHeavyAttack` _heavychainattack)
      (`/Engine/EditorBlueprintResources/StandardMacros.IncrementInt` _heavychainattack))
    (:`2`
      (`Character.PlayAnimMontage` _charref _output 1.0 "None")
      (`self.ComboHeavyAttack` _heavychainattack)
      (`/Engine/EditorBlueprintResources/StandardMacros.IncrementInt` _heavychainattack))
    (:`3`
      (`Character.PlayAnimMontage` _charref _output 1.0 "None")
      (`self.ComboHeavyAttack` _heavychainattack)
      (`/Engine/EditorBlueprintResources/StandardMacros.IncrementInt` _heavychainattack))))

(event `AttackTrace`
  ;[0.05098 0.05098 0.05098] Attack Trace
  (`|ExecutionSequence`
    (:`then_0`
      (`/Engine/EditorBlueprintResources/StandardMacros.DoOnce` false
        (:`Completed`
          (for _array_element (`|MakeArray` (`self.Collision`) (`self.Collision1`) (`self.Collision2`) (`self.Collision3`) (`self.Collision4`) (`self.Collision5`) (`self.Collision6`) (`self.Collision7`) (`self.Collision8`))
            (`KismetArrayLibrary.Array_Add` (`self.CollisionBoxes`) _array_element)))))
    (:`then_1`
      (for _array_element_2 (`self.CollisionBoxes`)
        (bind _returnvalue (`SceneComponent.K2_GetComponentLocation` _array_element_2))
        (bind (_outhit _returnvalue_2) (`KismetSystemLibrary.LineTraceSingleForObjects` _returnvalue (- _returnvalue (* (`KismetMathLibrary.GetForwardVector` (`SceneComponent.K2_GetComponentRotation` _array_element_2)) 5.0)) (`|MakeArray` "ObjectTypeQuery3" :!type "EObjectTypeQuery Enum") true (`|MakeArray` (`self.CharRef`) :!type "Actor Object Reference") "ForDuration" true (struct :`R` 1.0 :`A` 1.0) (struct :`G` 1.0 :`A` 1.0) 0.3))
        (if _returnvalue_2
          (`/Game/BluePrints/Player/Components/BPC_AttackSystem.Hit` (`/Game/BluePrints/Player/BP_PlayerCharacter.BPC_AttackSystem` (`self.CharRef`)) _outhit))))))

(fn `UserConstructionScript`)