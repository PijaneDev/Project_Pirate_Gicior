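; BP_PickUp is a pickup actor that offers an item to the player character through proximity.
; Its Sphere overlap events show the Widget on enter and hide it on exit, for any overlapping actor.
; For a BP_PlayerCharacter, both enter and exit write ItemToAdd into the equipment system's AttatchedWeapon, so leaving does not clear it.
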(event `self.Sphere.OnComponentBeginOverlap`
  (params (OverlappedComponent :type "PrimitiveComponent Object Reference") (OtherActor :type "Actor Object Reference") (OtherComp :type "PrimitiveComponent Object Reference") (OtherBodyIndex :type Integer) (bFromSweep :type Boolean) (SweepResult :type "HitResult Structure (by ref)"))
  (`SceneComponent.SetVisibility` (`self.Widget`) true false)
  (bind _asbp_player_character (cast `/Game/BluePrints/Player/BP_PlayerCharacter` OtherActor))
  (set `/Game/BluePrints/Player/Components/BPC_EquipmentSystem.AttatchedWeapon` (`self.ItemToAdd`) (`/Game/BluePrints/Player/BP_PlayerCharacter.BPC_EquipmentSystem` _asbp_player_character)))

(event `self.Sphere.OnComponentEndOverlap`
  (params (OverlappedComponent :type "PrimitiveComponent Object Reference") (OtherActor :type "Actor Object Reference") (OtherComp :type "PrimitiveComponent Object Reference") (OtherBodyIndex :type Integer))
  (`SceneComponent.SetVisibility` (`self.Widget`) false false)
  (bind _asbp_player_character (cast `/Game/BluePrints/Player/BP_PlayerCharacter` OtherActor))
  (set `/Game/BluePrints/Player/Components/BPC_EquipmentSystem.AttatchedWeapon` (`self.ItemToAdd`) (`/Game/BluePrints/Player/BP_PlayerCharacter.BPC_EquipmentSystem` _asbp_player_character)))

(fn `UserConstructionScript`)