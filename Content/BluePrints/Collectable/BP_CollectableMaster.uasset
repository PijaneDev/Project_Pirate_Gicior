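; Master Blueprint for collectable actors that destroy themselves when anything begins overlapping their Collision component.
; On destruction it sets IsDestroyed and passes itself to BP_GameState through CallCollectableDestroyed.
; BeginPlay destroys the actor immediately if IsDestroyed is already set.
; A MoveUpDown timeline would bob the mesh along relative Z, but nothing in this graph starts it.
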(event `self.ReceiveBeginPlay`
  (if (`self.isDestroyed?`)
    (`self.K2_DestroyActor` :!label _label)))

(event `self.Collision.OnComponentBeginOverlap`
  (params (OverlappedComponent :type "PrimitiveComponent Object Reference") (OtherActor :type "Actor Object Reference") (OtherComp :type "PrimitiveComponent Object Reference") (OtherBodyIndex :type Integer) (bFromSweep :type Boolean) (SweepResult :type "HitResult Structure (by ref)"))
  (goto _label))

(event `self.ReceiveDestroyed`
  (set `self.isDestroyed?` true)
  (bind _asbp_game_state (cast `/Game/BluePrints/BP_GameState` (`GameplayStatics.GetGameState`)))
  (`/Game/BluePrints/BP_GameState.CollectableDestroyed` _asbp_game_state self))

(fn `UserConstructionScript`)