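; BP_Sword is a sword weapon Blueprint that handles combo chain bookkeeping and starts its attack trace.
; The light and heavy combo events switch on the chain index, and each handled step zeroes the opposite chain counter on the character's BPCAttackSystem component.
; All handled steps behave identically, with no step-specific attack logic in this graph.
; AttackTraceInit simply calls WeaponAttackTrace, and the construction script is empty.
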(event `self.ComboLightAttack`
  (params (ChainLightAttack :type Integer))
  (bind _bpc_attacksystem (`/Game/BluePrints/Player/BP_PlayerCharacter.BPC_AttackSystem` (`self.CharRef`)))
  (switch `int` ChainLightAttack
    (:`0`
      (set `/Game/BluePrints/Player/Components/BPC_AttackSystem.HeavyChainAttack` 0 _bpc_attacksystem))
    (:`1`
      (set `/Game/BluePrints/Player/Components/BPC_AttackSystem.HeavyChainAttack` 0 _bpc_attacksystem))
    (:`2`
      (set `/Game/BluePrints/Player/Components/BPC_AttackSystem.HeavyChainAttack` 0 _bpc_attacksystem))))

(event `self.ComboHeavyAttack`
  (params (ChainHeavyAttack :type Integer))
  (bind _bpc_attacksystem (`/Game/BluePrints/Player/BP_PlayerCharacter.BPC_AttackSystem` (`self.CharRef`)))
  (switch `int` ChainHeavyAttack
    (:`0`
      (set `/Game/BluePrints/Player/Components/BPC_AttackSystem.LightChainAttack` 0 _bpc_attacksystem))
    (:`1`
      (set `/Game/BluePrints/Player/Components/BPC_AttackSystem.LightChainAttack` 0 _bpc_attacksystem))
    (:`2`
      (set `/Game/BluePrints/Player/Components/BPC_AttackSystem.LightChainAttack` 0 _bpc_attacksystem))))

(event `AttackTraceInit`
  (`self.WeaponAttackTrace`))

(fn `UserConstructionScript`)