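; Pickup actor that represents the item class set in ItemToAdd and shows a widget while something overlaps its sphere.
; The construction script uses that class's display name as the DT_Items row key and applies the row's static mesh and three skeletal meshes.
; Sphere begin and end overlap toggle the widget without filtering the overlapping actor.
; GetClassName exposes the same name key; adding the item is not handled here.
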(event `self.Sphere.OnComponentBeginOverlap`
  (params (OverlappedComponent :type "PrimitiveComponent Object Reference") (OtherActor :type "Actor Object Reference") (OtherComp :type "PrimitiveComponent Object Reference") (OtherBodyIndex :type Integer) (bFromSweep :type Boolean) (SweepResult :type "HitResult Structure (by ref)"))
  (`SceneComponent.SetVisibility` (`self.Widget`) true false))

(event `self.Sphere.OnComponentEndOverlap`
  (params (OverlappedComponent :type "PrimitiveComponent Object Reference") (OtherActor :type "Actor Object Reference") (OtherComp :type "PrimitiveComponent Object Reference") (OtherBodyIndex :type Integer))
  (`SceneComponent.SetVisibility` (`self.Widget`) false false))

(fn `GetClassName`
  (returns (ClassName :type Name))
  (return (`KismetStringLibrary.Conv_StringToName` (`KismetSystemLibrary.GetClassDisplayName` (`self.ItemToAdd`)))))

(fn `UserConstructionScript`
  (bind _returnvalue (`|GetDataTableRow` "/Game/BluePrints/DataTables/DT_Items.DT_Items" (`KismetStringLibrary.Conv_StringToName` (`KismetSystemLibrary.GetClassDisplayName` (`self.ItemToAdd`))))
    (:`then`
      (bind ((`StaticMesh_33_2D8470DE44547CD9DDC73B932F4940B8` _staticmesh) (`SkeletalMesh_38_CEC1DFDD4F0855D194813AB11BE4A261` _skeletalmesh) (`SkeletalMesh1_39_C31BADA946611F3CFA256D908C239185` _skeletalmesh1) (`SkeletalMesh2_40_EBE36AB94E5AC337846E2C83FE92C6FF` _skeletalmesh2)) (break `/Game/BluePrints/Structures/S_ItemInfo` _returnvalue))
      (`StaticMeshComponent.SetStaticMesh` (`self.StaticMesh`) _staticmesh)
      (`SkeletalMeshComponent.SetSkeletalMeshAsset` (`self.SkeletalMesh`) _skeletalmesh)
      (`SkeletalMeshComponent.SetSkeletalMeshAsset` (`self.SkeletalMesh1`) _skeletalmesh1)
      (`SkeletalMeshComponent.SetSkeletalMeshAsset` (`self.SkeletalMesh2`) _skeletalmesh2))))