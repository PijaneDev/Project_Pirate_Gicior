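; BP_Equipment is an equipment item Blueprint whose visuals come from data rather than being set per item.
; Its construction script looks up the row named by the item's data table handle in ItemData.
; A Static flag in that row selects between filling a single static mesh component and filling three skeletal mesh components with the row's assets.
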(fn `UserConstructionScript`
  (bind _itemdata (`self.ItemData`))
  (bind _returnvalue (`|GetDataTableRow` (break `DataTableRowHandle` (break `/Game/BluePrints/Structures/S_Slots` _itemdata)) (`.RowName` (break `DataTableRowHandle` (break `/Game/BluePrints/Structures/S_Slots` _itemdata))))
    (:`then`
      (bind ((`StaticMesh_12_DA5CEF7F45C0DE2B8F0A0DA317F3AEF1` _staticmesh) (`Socket_51_EA2B3B0F4C54C6F6C23FB3A2481D32B7` _socket) (`SkeletalMesh_36_4E551BB64E9561EA555208B6CB5D02D3` _skeletalmesh) (`SkeletalMesh2_38_03F1A6CF442EC61B4FF62DBC8C113553` _skeletalmesh2) (`SkeletalMesh3_41_D36A53ED418490100D5E58A2EAEF06E1` _skeletalmesh3) (`Static_44_F6F346CB424472C5C3FB01B3EE0FB065` _static)) (break `/Game/BluePrints/Structures/S_Equipment` _returnvalue))
      (if _static
        (`StaticMeshComponent.SetStaticMesh` (`self.StaticMesh`) _staticmesh)
        (else
          (`SkeletalMeshComponent.SetSkeletalMeshAsset` (`self.SkeletalMesh1`) _skeletalmesh)
          (`SkeletalMeshComponent.SetSkeletalMeshAsset` (`self.SkeletalMesh2`) _skeletalmesh2)
          (`SkeletalMeshComponent.SetSkeletalMeshAsset` (`self.SkeletalMesh3`) _skeletalmesh3))))))