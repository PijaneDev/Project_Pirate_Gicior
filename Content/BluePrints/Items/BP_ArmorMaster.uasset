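; BP_ArmorMaster is a master Blueprint for armor items that takes its visuals from a data table.
; The construction script calls Initalize, which looks up the row referenced by ItemData and stores it as ItemInfo.
; The row's Static flag selects between setting one static mesh and filling three skeletal mesh components.
; GetArmorRef returns the armor itself as a reference.
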(fn `GetArmorRef`
  (returns (ArmorRef :type "/Game/BluePrints/Items/BP_ArmorMaster Object Reference"))
  (return self))

(fn `Initalize`
  (bind _itemdata (`self.ItemData`))
  (`/Engine/EditorBlueprintResources/StandardMacros.IsValid` (break `DataTableRowHandle` (break `/Game/BluePrints/Structures/S_Slots` _itemdata))
    (:`Is Valid`
      (bind _returnvalue (`|GetDataTableRow` (break `DataTableRowHandle` (break `/Game/BluePrints/Structures/S_Slots` _itemdata)) (`.RowName` (break `DataTableRowHandle` (break `/Game/BluePrints/Structures/S_Slots` _itemdata))))
        (:`then`
          (bind _output_get (set `self.ItemInfo` _returnvalue))
          (if (`.Static_44_F6F346CB424472C5C3FB01B3EE0FB065` (break `/Game/BluePrints/Structures/S_Equipment` _output_get))
            (`StaticMeshComponent.SetStaticMesh` (`self.StaticMesh`) (`.StaticMesh_12_DA5CEF7F45C0DE2B8F0A0DA317F3AEF1` (break `/Game/BluePrints/Structures/S_Equipment` _output_get)))
            (else
              (`SkeletalMeshComponent.SetSkeletalMeshAsset` (`self.SkeletalMesh1`) (`.SkeletalMesh_36_4E551BB64E9561EA555208B6CB5D02D3` (break `/Game/BluePrints/Structures/S_Equipment` _output_get)))
              (`SkeletalMeshComponent.SetSkeletalMeshAsset` (`self.SkeletalMesh2`) (`.SkeletalMesh2_38_03F1A6CF442EC61B4FF62DBC8C113553` (break `/Game/BluePrints/Structures/S_Equipment` _output_get)))
              (`SkeletalMeshComponent.SetSkeletalMeshAsset` (`self.SkeletalMesh3`) (`.SkeletalMesh3_41_D36A53ED418490100D5E58A2EAEF06E1` (break `/Game/BluePrints/Structures/S_Equipment` _output_get))))))))))

(fn `UserConstructionScript`
  (`self.Initalize`))