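; BP_PushBarrel is a barrel that the player pushes a set distance along the X axis by bumping into it.
; On Hit, CanPush confirms the player faces the barrel and stands on a floor, then capsule-traces for obstacles in the push direction.
; A valid push disables player movement, attaches the player, plays a montage and slides the barrel with the MoveBlock timeline, then detaches and restores walking.
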(event `self.ReceiveHit`
  (params (MyComp :type "PrimitiveComponent Object Reference") (Other :type "Actor Object Reference") (OtherComp :type "PrimitiveComponent Object Reference") (bSelfMoved :type Boolean) (HitLocation :type "Vector Structure") (HitNormal :type "Vector Structure") (NormalImpulse :type "Vector Structure") (Hit :type "HitResult Structure (by ref)"))
  (bind _returnvalue_x (`KismetMathLibrary.BreakVector` (`self.GetActorForwardVector` Other)))
  (bind _returnvalue (`GameplayStatics.GetPlayerCharacter` 0))
  (if (== Other (`GameplayStatics.GetPlayerCharacter` 0))
    (set `self.PushDirection` (`KismetMathLibrary.Round` _returnvalue_x))
    (bind _canpush_ (`self.canPush?`))
    (if _canpush_
      (`CharacterMovementComponent.DisableMovement` (`Character.CharacterMovement` _returnvalue))
      (`self.K2_AttachToActor` _returnvalue self "None" "KeepWorld" "KeepWorld" "KeepWorld" true)
      (`self.Push`)
      (`|PlayMontage` (`Character.Mesh` _returnvalue) "/Game/Animations/Player/Push_UE_Montage.Push_UE_Montage"))))

(event `Push`
  (bind (_returnvalue_x _returnvalue_y _returnvalue_z) (`KismetMathLibrary.BreakVector` (+ (0.0 0.0 0.0) (`self.CurrentLocation`))))
  (set `self.CurrentLocation` (`self.K2_GetActorLocation`))
  (bind (_direction _position) (`Timeline|MoveBlock` :!via `PlayFromStart`)
    (:`Update`
      (`self.K2_SetActorRelativeLocation` (`KismetMathLibrary.MakeVector` (+ (* _position (`self.PushDirection`) (`self.TravelDistance`)) _returnvalue_x) _returnvalue_y _returnvalue_z)))
    (:`Finished`
      (`self.StopPushing`))))

(event `StopPushing`
  (bind _returnvalue (`GameplayStatics.GetPlayerCharacter` 0))
  (`CharacterMovementComponent.SetMovementMode` (`Character.CharacterMovement` _returnvalue) "MOVE_Walking" 0)
  (`self.K2_DetachFromActor` _returnvalue "KeepWorld" "KeepWorld" "KeepWorld"))

(fn `canPush?`
  (returns (`CanPush?` :type Boolean))
  (bind _returnvalue (`GameplayStatics.GetPlayerCharacter` 0))
  (bind _returnvalue_2 (+ (`self.K2_GetActorLocation`) (0.0 0.0 50.0)))
  (bind _returnvalue_3 (- (`self.K2_GetActorLocation` _returnvalue) (0.0 0.0 50.0)))
  (bind _returnvalue_x (`KismetMathLibrary.BreakVector` (* (`self.GetActorForwardVector` (`GameplayStatics.GetPlayerCharacter` 0)) 80.0)))
  (bind (_outhit _returnvalue_4) (`KismetSystemLibrary.LineTraceSingle` _returnvalue_3 (+ _returnvalue_3 (* (`self.GetActorForwardVector` _returnvalue) 100.0)) "TraceTypeQuery1" false (`|MakeArray` _returnvalue :!type "Actor Object Reference") "ForDuration" false (struct :`R` 1.0 :`A` 1.0) (struct :`G` 1.0 :`A` 1.0) 2.0))
  (if _returnvalue_4
    (if (== (`.HitActor` (`GameplayStatics.BreakHitResult` _outhit)) self)
      (if (`.bBlockingHit` (break `FindFloorResult` (`CharacterMovementComponent.CurrentFloor` (`Character.CharacterMovement` (`GameplayStatics.GetPlayerCharacter` 0)))))
        (bind (_outhit_2 _returnvalue_5) (`KismetSystemLibrary.CapsuleTraceSingle` :`Start` _returnvalue_2 :`End` (+ _returnvalue_2 (`KismetMathLibrary.MakeVector` _returnvalue_x)) :`Radius` 20.0 :`TraceChannel` "TraceTypeQuery1" :`DrawDebugType` "ForDuration" :`DrawTime` 2.0))
        (if _returnvalue_5
          (return false)
          (else
            (return true)))
        (else
          (return false)))
      (else
        (return false)))))

(fn `UserConstructionScript`)