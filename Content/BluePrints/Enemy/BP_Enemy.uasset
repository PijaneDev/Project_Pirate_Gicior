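; BP_Enemy is a zombie enemy character that takes damage, reacts to hits, attacks and dies.
; Damage goes to BPCEnemyStats; non-lethal hits play a reaction montage and launch it along the player's forward vector.
; On death it hides its bar, disables capsule collision, notifies its AI controller and waits out the death montage.
; A timeline then drives BPCDissolveComponent and offsets the mesh vertically before destroying the actor.
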(event `self.ReceiveBeginPlay`
  (`/Game/BluePrints/Enemy/BPC_EnemyStats.Initalize` (`self.BPC_EnemyStats`)))

(event `self.ReceiveAnyDamage`
  (params (Damage :type "Float (single-precision)") (DamageType :type "DamageType Object Reference") (InstigatedBy :type "Controller Object Reference") (DamageCauser :type "Actor Object Reference"))
  (bind (_meshlocation_x _meshlocation_y _meshlocation_z) (`KismetMathLibrary.BreakVector` (`self.MeshLocation`)))
  (bind _death_ (`/Game/BluePrints/Enemy/BPC_EnemyStats.DecreaseHealth` (`self.BPC_EnemyStats`) Damage))
  (if _death_
    (bind _animtime (`self.Death`))
    (`KismetSystemLibrary.Delay` _animtime)
    (set `self.MeshLocation` (`SceneComponent.RelativeLocation` (`self.Mesh`)))
    (bind (_direction _dissolvevalue _offsetvalue) (`Timeline|DissolveTimeline` :!via `PlayFromStart`)
      (:`Update`
        (`/Game/BluePrints/Enemy/BPC_DissolveComponent.SetDissolvePercent` (`self.BPC_DissolveComponent`) _dissolvevalue)
        (`SceneComponent.K2_SetRelativeLocation` (`self.Mesh`) (`KismetMathLibrary.MakeVector` _meshlocation_x _meshlocation_y (+ _meshlocation_z _offsetvalue)) false false))
      (:`Finished`
        (`self.K2_DestroyActor`)))
    (else
      (`self.PlayAnimMontage` "/Game/Animations/Enemies/Enemy/animsX/Zombie_Reaction_Hit_Montage.Zombie_Reaction_Hit_Montage")
      (bind _asbp_third_person_character (cast `/Game/BluePrints/Player/BP_ThirdPersonCharacter` (`GameplayStatics.GetPlayerCharacter` 0)))
      (`self.LaunchCharacter` (* (`KismetMathLibrary.GetForwardVector` (`self.K2_GetActorRotation` _asbp_third_person_character)) 125.0)))))

(fn `Attack`
  (returns (AnimationDuration :type "Float (double-precision)"))
  (bind _returnvalue (`self.PlayAnimMontage` "/Game/Animations/Enemies/Enemy/animsX/zombie_attack11_Montage.zombie_attack11_Montage"))
  (return _returnvalue))

(fn `Death`
  (returns (AnimTime :type "Float (single-precision)"))
  (`SceneComponent.SetVisibility` (`self.Bar`) false false)
  (`PrimitiveComponent.SetCollisionEnabled` (`self.CapsuleComponent`) "NoCollision")
  (bind _asbp_aicontroller_generic (cast `/Game/AI/BP_AIController_Generic` (`self.GetController`)))
  (`/Game/AI/BP_AIController_Generic.Death` _asbp_aicontroller_generic)
  (bind _returnvalue (`self.PlayAnimMontage` "/Game/Animations/Enemies/Enemy/animsX/zombie_death_Montage.zombie_death_Montage"))
  (return _returnvalue))

(fn `Hit`)

(fn `UserConstructionScript`)