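; Actor component that tracks health for BP_Enemy and drives its health bar widget.
; Initalize casts the owner to BP_Enemy and caches the progress bar from the WB_AIHealthBar widget on its Bar component.
; DecreaseHealth subtracts damage, clamps at zero and returns true once health is depleted.
; Each change refreshes the bar through UpdateHealthBar as the ratio of current to max health.
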(event `Initalize`
  (bind _asbp_enemy (cast `/Game/BluePrints/Enemy/BP_Enemy` (`self.GetOwner`)))
  (bind _aswb_aihealth_bar (cast `/Game/UI/MainGame/WB_AIHealthBar` (`WidgetComponent.GetWidget` (`/Game/BluePrints/Enemy/BP_Enemy.Bar` _asbp_enemy))))
  (set `self.Health Bar` (`/Game/UI/MainGame/WB_AIHealthBar.HealthBar` _aswb_aihealth_bar))
  (`self.UpdateHealthBar`))

(fn `DecreaseHealth`
  (params (Damage :type "Float (double-precision)"))
  (returns (`Death?` :type Boolean))
  (bind _returnvalue (- (`self.CurrentHealth`) Damage))
  (if (> _returnvalue 0.0)
    (set `self.CurrentHealth` _returnvalue)
    (`self.UpdateHealthBar`)
    (return false)
    (else
      (set `self.CurrentHealth` 0.0)
      (`self.UpdateHealthBar`)
      (return true))))

(fn `UpdateHealthBar`
  (`ProgressBar.SetPercent` (`self.Health Bar`) (/ (`self.CurrentHealth`) (`self.MaxHealth`))))