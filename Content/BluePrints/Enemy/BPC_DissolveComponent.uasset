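; Actor component that lets its owning enemy dissolve by driving a scalar parameter on its materials.
; On BeginPlay it gathers every static and skeletal mesh component on the owner and swaps each material slot for a dynamic material instance, caching them all in one array.
; SetDissolvePercent then pushes the given value into the DissolveAmount parameter on every cached instance.
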(event `self.ReceiveBeginPlay`
  (bind _returnvalue (`self.GetOwner`))
  (`self.GetMeshFromMaterials` (`Actor.K2_GetComponentsByClass` _returnvalue "/Script/Engine.StaticMeshComponent") (`Actor.K2_GetComponentsByClass` _returnvalue "/Script/Engine.SkeletalMeshComponent")))

(event `SetDissolvePercent`
  (params (DissolvePercent :type "Float (double-precision)"))
  (for _array_element (`self.MaterialsToDissolve`)
    (`MaterialInstanceDynamic.SetScalarParameterValue` _array_element "DissolveAmount" DissolvePercent)))

(fn `GetMeshFromMaterials`
  (params (StaticMesh :type "Array of StaticMeshComponent Object Reference") (SkeletalMesh :type "Array of SkeletalMeshComponent Object Reference"))
  (`|ExecutionSequence`
    (:`then_0`
      (for _array_element StaticMesh
        (for (_array_element_2 _array_index) (`MeshComponent.GetMaterials` _array_element)
          (bind _returnvalue (`KismetMaterialLibrary.CreateDynamicMaterialInstance` _array_element_2))
          (`PrimitiveComponent.SetMaterial` _array_element _array_index _returnvalue)
          (`KismetArrayLibrary.Array_Add` (`self.MaterialsToDissolve`) _returnvalue))))
    (:`then_1`
      (for _array_element_3 SkeletalMesh
        (for (_array_element_4 _array_index_2) (`MeshComponent.GetMaterials` _array_element_3)
          (bind _returnvalue_2 (`KismetMaterialLibrary.CreateDynamicMaterialInstance` _array_element_4))
          (`PrimitiveComponent.SetMaterial` _array_element_3 _array_index_2 _returnvalue_2)
          (`KismetArrayLibrary.Array_Add` (`self.MaterialsToDissolve`) _returnvalue_2))))))