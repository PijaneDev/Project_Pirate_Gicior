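; Generic AI controller that runs BT_AI on BeginPlay and feeds perception results into its blackboard.
; Perception updates go through SightDetection, which sets TargetActor on successful sight and clears it on any other stimulus, hearing included.
; They then go through HearingDetection, which writes the location of hearing stimuli to InvestigationLocation.
; A Death event detaches the controlled pawn from the controller pending destroy.
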(event `self.ReceiveBeginPlay`
  (`self.RunBehaviorTree` "/Game/AI/BT_AI.BT_AI"))

(event `self.AIPerception.OnTargetPerceptionUpdated`
  (params (Actor :type "Actor Object Reference") (Stimulus :type "AIStimulus Structure"))
  (`self.SightDetection` Actor Stimulus)
  (`self.HearingDetection` Actor Stimulus))

(event `Death`
  (`Pawn.DetachFromControllerPendingDestroy` (`self.K2_GetPawn`)))

(fn `HearingDetection`
  (params (Actor :type "Actor Object Reference") (Stimulus :type "AIStimulus Structure"))
  (bind _returnvalue (`AIPerceptionSystem.GetSenseClassForStimulus` Stimulus))
  (if (== _returnvalue "/Script/AIModule.AISense_Hearing")
    (`BlackboardComponent.SetValueAsVector` (`self.Blackboard`) "InvestigationLocation" (`.StimulusLocation` (break `AIStimulus` Stimulus)))))

(fn `SightDetection`
  (params (Actor :type "Actor Object Reference") (Stimulus :type "AIStimulus Structure"))
  (bind _returnvalue (`AIPerceptionSystem.GetSenseClassForStimulus` Stimulus))
  (if (and (== _returnvalue "/Script/AIModule.AISense_Sight") (`.bSuccessfullySensed` (break `AIStimulus` Stimulus)))
    (`BlackboardComponent.SetValueAsObject` (`AIBlueprintHelperLibrary.GetBlackboard` null) "TargetActor" Actor)
    (else
      (`BlackboardComponent.SetValueAsObject` (`AIBlueprintHelperLibrary.GetBlackboard` null) "TargetActor" null))))

(fn `UserConstructionScript`)